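; BP_UHL_TestPawn is a test AI pawn that runs a behavior tree and reacts to sighted actors.
; On BeginPlay it starts its BehaviorTree through its AI controller.
; When AI perception updates and sight is enabled, sight stimuli write the perceived actor into the blackboard enemy key, without checking whether it was sensed or lost.
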(event OnTargetPerceptionUpdated(AIPerception)
  (params (Actor :type Actor%20Object%20Reference) (Stimulus :type AI%20Stimulus%20Structure))
  (if (Variables|Default|GetbSightSenseEnabled)
    (bind _returnvalue (Class|AIPerceptionSystem|GetSenseClassforStimulus Stimulus))
    (if (== _returnvalue "/Script/AIModule.AISense_Sight")
      (AI|Components|Blackboard|SetValueasObject (AI|GetBlackboard 0) (Variables|Default|GetBBKey_Enemy) Actor))))

(event EventBeginPlay
  (AI|RunBehaviorTree (AI|GetAIController self) (Variables|Default|GetBehaviorTree)))

(event Collision|EventActorBeginOverlap
  (params (OtherActor :type Actor%20Object%20Reference)))

(event EventTick
  (params (DeltaSeconds :type Float%20%28single-precision%29)))

(fn ConstructionScript)