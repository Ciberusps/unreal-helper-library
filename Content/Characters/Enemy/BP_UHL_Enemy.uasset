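; Enemy character Blueprint that runs a behavior tree and feeds sight perception into its blackboard.
; BeginPlay starts the tree on its AI controller and adds replicated loose gameplay tags.
; When sight is enabled, sight perception updates write the actor to the enemy key, without checking whether it was sensed or lost.
; A one-shot timer prints debug strings if the ability system holds a test tag.
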(event OnTargetPerceptionUpdated(AIPerception)
  (params (Actor :type Actor%20Object%20Reference) (Stimulus :type AI%20Stimulus%20Structure))
  (if (Variables|Default|GetbSightSenseEnabled)
    (bind _returnvalue (Class|AIPerceptionSystem|GetSenseClassforStimulus Stimulus))
    (if (== _returnvalue "/Script/AIModule.AISense_Sight")
      (AI|Components|Blackboard|SetValueasObject (AI|GetBlackboard 0) (Variables|Default|GetBBKey_Enemy) Actor))))

(event Custom|CustomEvent
  (if (GameplayTags|HasMatchingGameplayTag (Variables|Default|GetAbilitySystem) "(TagName=\"Tests.GenericTag\")")
    (Class|UnrealHelperLibraryBPLibrary|DebugPrintStrings "" "" "" "" "" "" "" "" "" "" 5.0 true)))

(event EventBeginPlay
  (|CallParentFunction)
  (AI|RunBehaviorTree (AI|GetAIController self) (Variables|Default|GetBehaviorTree))
  (Ability|GameplayEffect|AddLooseGameplayTags self (Variables|Default|GetGameplay%20Tags) true)
  (Utilities|Time|SetTimerbyEvent (delegate Custom|CustomEvent) 2.0))

(fn ConstructionScript
  (|CallParentFunction))