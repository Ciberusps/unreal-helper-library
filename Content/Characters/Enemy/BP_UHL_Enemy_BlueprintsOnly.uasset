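; Enemy character Blueprint built on UHL's ability system, set up entirely in Blueprints as its name suggests.
; On BeginPlay it initializes the UHLAbilitySystem component with its controller as owner and activates the initial abilities.
; The construction script runs the parent's, then writes the TextAboveHead value to a TextRender label.
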(event EventBeginPlay
  (Class|UHLAbilitySystemComponent|InitAbilitySystem (Variables|Default|GetUHLAbilitySystem) (Pawn|GetController) 0 true))

(fn ConstructionScript
  (|CallParentFunction)
  (Rendering|Components|TextRender|SetText (Variables|Default|GetTextRender) (Utilities|Text|ToText(String) (Variables|Default|GetTextAboveHead))))