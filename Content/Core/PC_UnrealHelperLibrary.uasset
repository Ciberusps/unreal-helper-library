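; Player controller for the UnrealHelperLibrary project that toggles a debug menu through the IA_DebugMenu Enhanced Input action.
; The UI_DebugMenu widget is created and added to the viewport on first press, then reused.
; A FlipFlop alternates each press between showing and collapsing the menu, switching input mode, game pause and mouse cursor visibility along with it.
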(event Input|EnhancedActionEvents|EnhancedInputActionIA_DebugMenu
  (params (ActionValue :type Boolean) (ElapsedSeconds :type Float%20%28double-precision%29) (TriggeredSeconds :type Float%20%28double-precision%29) (InputAction :type Input%20Action%20Object%20Reference :default "/UnrealHelperLibrary/Input/Actions/IA_DebugMenu.IA_DebugMenu"))
  (Utilities|IsValid (Variables|Default|GetUI_DebugMenu)
    (:Is%20Valid
      _)
    (:Is%20Not%20Valid
      (bind _returnvalue (UserInterface|CreateWidget "/UnrealHelperLibrary/UI/UI_DebugMenu.UI_DebugMenu_C" self))
      (bind _output_get (Variables|Default|SetUI_DebugMenu _returnvalue))
      (UserInterface|Viewport|AddtoViewport _output_get 0)))
  (bind _isa (Utilities|FlowControl|FlipFlop)
    (:A
      (Input|SetInputModeGameandUI self (Variables|Default|GetUI_DebugMenu) "DoNotLock" true false))
    (:B
      (Input|SetInputModeGameOnly self false)))
  (Game|SetGamePaused _isa)
  (Variables|Default|SetbShowMouseCursor _isa)
  (Widget|SetVisibility (Variables|Default|GetUI_DebugMenu) (select _isa "Visible" "Collapsed")))

(event EventBeginPlay)

(event EventTick
  (params (DeltaSeconds :type Float%20%28single-precision%29)))

(fn ConstructionScript)