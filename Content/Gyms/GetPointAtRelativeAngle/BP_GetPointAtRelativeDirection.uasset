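; Gym test actor that exercises GetPointAtRelativeDirection, a function defined outside this graph.
; On BeginPlay it calls the function for the four cardinal and four diagonal relative directions, all at the same distance, with debug enabled and a distinct color for each.
; Each result overwrites a single TestVar that is never read, and the construction script, Tick and overlap events are empty.
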(event EventBeginPlay
  (Variables|Default|SetTestVar (Class|UnrealHelperLibraryBPL|GetPointatRelativeDirection 0 "Front" 5e+02 true -1.0 "(R=1.000000,G=0.000000,B=0.003677,A=1.000000)"))
  (Variables|Default|SetTestVar (Class|UnrealHelperLibraryBPL|GetPointatRelativeDirection 0 "Back" 5e+02 true -1.0 "(R=0.009721,G=0.000000,B=1.000000,A=1.000000)"))
  (Variables|Default|SetTestVar (Class|UnrealHelperLibraryBPL|GetPointatRelativeDirection 0 "Left" 5e+02 true -1.0 "(R=0.000000,G=1.000000,B=0.076185,A=1.000000)"))
  (Variables|Default|SetTestVar (Class|UnrealHelperLibraryBPL|GetPointatRelativeDirection 0 "Right" 5e+02 true -1.0 "(R=0.938686,G=1.000000,B=0.000000,A=1.000000)"))
  (Variables|Default|SetTestVar (Class|UnrealHelperLibraryBPL|GetPointatRelativeDirection 0 "FrontLeft" 5e+02 true -1.0 "(R=1.000000,G=0.491021,B=0.000000,A=1.000000)"))
  (Variables|Default|SetTestVar (Class|UnrealHelperLibraryBPL|GetPointatRelativeDirection 0 "FrontRight" 5e+02 true -1.0 "(R=1.000000,G=0.000000,B=0.672443,A=1.000000)"))
  (Variables|Default|SetTestVar (Class|UnrealHelperLibraryBPL|GetPointatRelativeDirection 0 "BackLeft" 5e+02 true -1.0 "(R=0.000000,G=1.000000,B=0.982251,A=1.000000)"))
  (Variables|Default|SetTestVar (Class|UnrealHelperLibraryBPL|GetPointatRelativeDirection 0 "BackRight" 5e+02 true -1.0 "(R=0.318547,G=0.006995,B=0.000000,A=1.000000)")))

(event Collision|EventActorBeginOverlap
  (params (OtherActor :type Actor%20Object%20Reference)))

(event EventTick
  (params (DeltaSeconds :type Float%20%28single-precision%29)))

(fn ConstructionScript)